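; Player character Blueprint handling forward-only walking, look, crouch and a hold-to-show scope overlay.
; Forward input moves the character and starts a walk or crouch camera shake, with a flag preventing restarts.
; Releasing forward input, hits, and crouch toggles (after a short delay) stop all shakes, letting the matching one restart.
; Holding Scope creates a widget on the viewport, removed on release.
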(event Collision|EventHit
  (params (MyComp :type Primitive%20Component%20Object%20Reference) (Other :type Actor%20Object%20Reference) (OtherComp :type Primitive%20Component%20Object%20Reference) (bSelfMoved :type Boolean) (HitLocation :type Vector :default "0, 0, 0") (HitNormal :type Vector :default "0, 0, 0") (NormalImpulse :type Vector :default "0, 0, 0") (Hit :type Hit%20Result%20Structure%20%28by%20ref%29))
  ;[1 1 1] Stop
  (if (Variables|Default|GetIsShakePlaying)
    (CameraShake|StopAllCameraShakes (Game|GetPlayerCameraManager 0) true)
    (Variables|Default|SetIsShakePlaying false)))

(event Input|ActionEvents|InputActionCrouch
  (params (Key :type Key%20Structure))
  ;[1 1 1] Crouch
  (:Pressed
    (Character|Crouch)
    (Utilities|FlowControl|Delay 0.2 :!label _label)
    ;[1 1 1] Stop
    (if (Variables|Default|GetIsShakePlaying)
      (CameraShake|StopAllCameraShakes (Game|GetPlayerCameraManager 0) true)
      (Variables|Default|SetIsShakePlaying false)))
  (:Released
    (Character|UnCrouch)
    (goto _label)))

(event Input|ActionEvents|InputActionScope
  (params (Key :type Key%20Structure))
  ;[1 1 1] Scale
  (:Pressed
    (bind _returnvalue (UserInterface|CreateWidget "/Game/Resource/BluePrints/Scope.Scope_C"))
    (bind _output_get (Variables|Default|SetScope _returnvalue))
    (UserInterface|Viewport|AddtoViewport _output_get 0))
  (:Released
    (Widget|RemovefromParent (Variables|Default|GetScope))))

(event Input|AxisEvents|InputAxisMoveForward
  (params (AxisValue :type Float%20%28single-precision%29))
  ;[1 1 1] MoveForward
  (if (> AxisValue 0.0)
    ;[1 1 1] Walk
    (Pawn|Input|AddMovementInput (Transformation|GetActorForwardVector) 1.0 false)
    (if (not (Variables|Default|GetIsShakePlaying))
      ;[1 1 1] Choose Camera Shake
      (if (Variables|Default|GetbIsCrouched)
        (Variables|Default|SetCameraShake "/Game/Resource/BluePrints/CrouchCameraShake.CrouchCameraShake_C")
        (else
          (Variables|Default|SetCameraShake "/Game/Resource/BluePrints/WalkCameraShake.WalkCameraShake_C")))
      (Class|PlayerCameraManager|PlayCameraShake (Game|GetPlayerCameraManager 0) (Variables|Default|GetCameraShake) 1.0 "CameraLocal" "0, 0, 0")
      (Variables|Default|SetIsShakePlaying true))
    (else
      ;[1 1 1] Stop
      (if (Variables|Default|GetIsShakePlaying)
        (CameraShake|StopAllCameraShakes (Game|GetPlayerCameraManager 0) true)
        (Variables|Default|SetIsShakePlaying false)))))

(event Input|AxisEvents|InputAxisTurn
  (params (AxisValue :type Float%20%28single-precision%29))
  ;[1 1 1] Turn
  (Pawn|Input|AddControllerYawInput AxisValue))

(event Input|AxisEvents|InputAxisLookUp
  (params (AxisValue :type Float%20%28single-precision%29))
  ;[1 1 1] LookUp
  (Pawn|Input|AddControllerPitchInput AxisValue))

(fn ConstructionScript)